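; BallSpawner is a Pong actor that creates the arena and keeps balls in play.
; On BeginPlay it caches the BasePong game mode as GameState, spawns a PongArena that references it back, then spawns the first PongBall at its root location.
; BallSpawnCheck, not called within this Blueprint, decrements the live-ball count and spawns a replacement if the count is below MaxBalls and the game is not won.
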(event `self.ReceiveBeginPlay`
  (bind _asbase_pong (cast `/Game/Blueprints/BasePong` (`GameplayStatics.GetGameMode`)))
  (set `self.Game State` _asbase_pong)
  (bind _returnvalue (`|SpawnActorFromClass` "/Game/Blueprints/PongArena.PongArena_C" (`KismetMathLibrary.MakeTransform` (0.0 0.0 0.0)) "Undefined" "OverrideRootScale" null null))
  (bind _output_get (set `self.Current Arena` _returnvalue))
  (set `/Game/Blueprints/PongArena.BallSpawner` self _output_get)
  (`self.SpawnBall`))

(fn `BallSpawnCheck`
  (bind _result (`/Engine/EditorBlueprintResources/StandardMacros.DecrementInt` (`self.BallsInPlay`))
    (:`  `
      (bind _output_get (set `self.BallsInPlay` _result))
      (if (`/Game/Blueprints/BasePong.Game Won` (`self.Game State`))
        _
        (elif (< _output_get (`self.MaxBalls`))
          (`self.SpawnBall`))))))

(fn `SpawnBall`
  (`|SpawnActorFromClass` "/Game/Blueprints/PongBall.PongBall_C" (`KismetMathLibrary.MakeTransform` (`SceneComponent.K2_GetComponentLocation` (`self.DefaultSceneRoot`))) "Undefined" "OverrideRootScale" null null)
  (bind _result (`/Engine/EditorBlueprintResources/StandardMacros.IncrementInt` (`self.BallsInPlay`))
    (:`  `
      (set `self.BallsInPlay` _result))))

(fn `UserConstructionScript`)