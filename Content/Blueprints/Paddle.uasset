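; Paddle actor that the player drags by touch, moving in the Y-Z plane at a fixed X.
; A gate on Tick opens when a Touch1 press arrives and closes on any touch release.
; While open, it repeats the finger's screen trace as a Visibility line trace and sweeps the paddle to the hit's Y and Z.
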(event `self.ReceiveTick`
  (params (DeltaSeconds :type "Float (single-precision)"))
  (`/Engine/EditorBlueprintResources/StandardMacros.Gate` true :!label _label
    (:`Exit`
      (bind (_bblockinghit _binitialoverlap _time _distance _location _impactpoint _normal _impactnormal _physmat _hitactor _hitcomponent _hitbonename _hititem _faceindex _tracestart _traceend) (`GameplayStatics.BreakHitResult` (`PlayerController.GetHitResultUnderFingerByChannel` (`GameplayStatics.GetPlayerController` 0) (stale `InputTouch` FingerIndex) "TraceTypeQuery1" true)))
      (bind _outhit (`KismetSystemLibrary.LineTraceSingle` :`Start` _tracestart :`End` _traceend :`TraceChannel` "TraceTypeQuery1" :`bIgnoreSelf` false))
      (`self.K2_SetActorLocation` (`KismetMathLibrary.MakeVector` (.x (`self.K2_GetActorLocation` self)) (.y (`.Location` (`GameplayStatics.BreakHitResult` _outhit))) (.z (`.Location` (`GameplayStatics.BreakHitResult` _outhit)))) true))))

(event `InputTouch`
  (params (Location :type "Vector Structure") (FingerIndex :type "ETouchIndex Enum"))
  (:`Pressed`
    (if (`|EnumEquality` FingerIndex "Touch1")
      (goto _label :!via `Open`)))
  (:`Released`
    (goto _label :!via `Close`)))

(fn `UserConstructionScript`)