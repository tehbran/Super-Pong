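; BasePong runs the match rules for a two-player Pong game with powerups, tracking scores and declaring a winner at 30 points.
; On BeginPlay it creates the BP_UI HUD, a ball spawner and six fixed-position powerup spawners, handing itself to the HUD and powerup spawners.
; Tick uses a random Delay as a repeating timer to trigger a random spawner when no powerup remains.
; Scoring updates the HUD, which shows the restart screen on a win.
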(event `self.ReceiveBeginPlay`
  (bind _returnvalue (`|CreateWidget` "/Game/Blueprints/BP_UI.BP_UI_C"))
  (`UserWidget.AddToViewport` _returnvalue 0)
  (set `/Game/Blueprints/BP_UI.GameVars` self _returnvalue)
  (set `self.HUDWidget` _returnvalue)
  (bind _returnvalue_2 (`|SpawnActorFromClass` "/Game/Blueprints/BallSpawner.BallSpawner_C" (`KismetMathLibrary.MakeTransform` (0.0 0.0 0.0)) "Undefined" "OverrideRootScale" null null))
  (set `self.ballSpawner` _returnvalue_2)
  (bind _returnvalue_3 (`|SpawnActorFromClass` "/Game/Blueprints/PowerupSpawner.PowerupSpawner_C" (`KismetMathLibrary.MakeTransform` (480.0 215.0 58.0)) "Undefined" "OverrideRootScale" null null))
  (bind _output_get (set `self.pSpawn1` _returnvalue_3))
  (set `/Game/Blueprints/PowerupSpawner.gameState` self _output_get)
  (bind _returnvalue_4 (`|SpawnActorFromClass` "/Game/Blueprints/PowerupSpawner.PowerupSpawner_C" (`KismetMathLibrary.MakeTransform` (355.0 -150.0 -120.0)) "Undefined" "OverrideRootScale" null null))
  (bind _output_get_2 (set `self.pSpawn2` _returnvalue_4))
  (set `/Game/Blueprints/PowerupSpawner.gameState` self _output_get_2)
  (bind _returnvalue_5 (`|SpawnActorFromClass` "/Game/Blueprints/PowerupSpawner.PowerupSpawner_C" (`KismetMathLibrary.MakeTransform` (130.0 -40.0 -25.0)) "Undefined" "OverrideRootScale" null null))
  (bind _output_get_3 (set `self.pSpawn3` _returnvalue_5))
  (set `/Game/Blueprints/PowerupSpawner.gameState` self _output_get_3)
  (bind _returnvalue_6 (`|SpawnActorFromClass` "/Game/Blueprints/PowerupSpawner.PowerupSpawner_C" (`KismetMathLibrary.MakeTransform` (-255.0 195.0 125.0)) "Undefined" "OverrideRootScale" null null))
  (bind _output_get_4 (set `self.pSpawn4` _returnvalue_6))
  (set `/Game/Blueprints/PowerupSpawner.gameState` self _output_get_4)
  (bind _returnvalue_7 (`|SpawnActorFromClass` "/Game/Blueprints/PowerupSpawner.PowerupSpawner_C" (`KismetMathLibrary.MakeTransform` (-195.0 -100.0 -90.0)) "Undefined" "OverrideRootScale" null null))
  (bind _output_get_5 (set `self.pSpawn5` _returnvalue_7))
  (set `/Game/Blueprints/PowerupSpawner.gameState` self _output_get_5)
  (bind _returnvalue_8 (`|SpawnActorFromClass` "/Game/Blueprints/PowerupSpawner.PowerupSpawner_C" (`KismetMathLibrary.MakeTransform` (-485.0 125.0 -145.0)) "Undefined" "OverrideRootScale" null null))
  (bind _output_get_6 (set `self.pSpawn6` _returnvalue_8))
  (set `/Game/Blueprints/PowerupSpawner.gameState` self _output_get_6)
  (`self.Spawn Random Powerup`))

(event `self.ReceiveTick`
  (params (DeltaSeconds :type "Float (single-precision)"))
  (`KismetSystemLibrary.Delay` (`KismetMathLibrary.RandomFloatInRange` 5.0 10.0))
  (if (< (`self.PowerupsOnField`) 1)
    (`self.Spawn Random Powerup`)))

(fn `DisplayRestart`
  (params (Winner :type String))
  (`/Game/Blueprints/BP_UI.RestartScreen` (`self.HUDWidget`) Winner))

(fn `P1 Scored`
  (bind _result (`/Engine/EditorBlueprintResources/StandardMacros.IncrementInt` (`self.P1 Score`))
    (:`  `
      (`/Game/Blueprints/BP_UI.Update Score` (`self.HUDWidget`))
      (if (== _result 30)
        (set `self.Game Won` true)
        (`self.DisplayRestart` "Player One Wins!")))))

(fn `P2 Scored`
  (bind _result (`/Engine/EditorBlueprintResources/StandardMacros.IncrementInt` (`self.P2 Score`))
    (:`  `
      (`/Game/Blueprints/BP_UI.Update Score` (`self.HUDWidget`))
      (if (== _result 30)
        (set `self.Game Won` true)
        (`self.DisplayRestart` "Player Two Wins!")))))

(fn `Spawn Random Powerup`
  (`/Game/Blueprints/PowerupSpawner.Spawn Random Power` (select `int` (`KismetMathLibrary.RandomIntegerInRange` 0 5) :`0` (`self.pSpawn1`) :`1` (`self.pSpawn2`) :`2` (`self.pSpawn3`) :`3` (`self.pSpawn4`) :`4` (`self.pSpawn5`) :`5` (`self.pSpawn6`)))
  (`/Engine/EditorBlueprintResources/StandardMacros.IncrementInt` (`self.PowerupsOnField`)))

(fn `UserConstructionScript`)