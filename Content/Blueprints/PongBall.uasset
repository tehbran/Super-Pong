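; PongBall is the ball actor for a Pong-style game, which can turn into a bomb through a power-up.
; On BeginPlay it launches its Sphere with an impulse whose direction is randomly positive or negative on each axis, at fixed magnitudes.
; Overlapping a BombPower actor calls BecomeBomb, which only sets the IsBomb flag; an attached emitter spawn there is left unconnected.
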(event `self.ReceiveBeginPlay`
  (`PrimitiveComponent.AddImpulse` (`self.Sphere`) (`KismetMathLibrary.MakeVector` (select `int` (`KismetMathLibrary.RandomIntegerInRange` 0 1) :`0` -300.0 :`1` 300.0 :!type "Float (single-precision)") (select `int` (`KismetMathLibrary.RandomIntegerInRange` 0 1) :`0` -300.0 :`1` 300.0 :!type "Float (single-precision)") (select `int` (`KismetMathLibrary.RandomIntegerInRange` 0 1) :`0` -250.0 :`1` 250.0 :!type "Float (single-precision)")) "None" false))

(event `self.Sphere.OnComponentBeginOverlap`
  (params (OverlappedComponent :type "PrimitiveComponent Object Reference") (OtherActor :type "Actor Object Reference") (OtherComp :type "PrimitiveComponent Object Reference") (OtherBodyIndex :type Integer) (bFromSweep :type Boolean) (SweepResult :type "HitResult Structure (by ref)"))
  (cast `/Game/Blueprints/BombPower` OtherActor)
  (`self.BecomeBomb`))

(fn `BecomeBomb`
  (set `self.isBomb` true))

(fn `UserConstructionScript`)