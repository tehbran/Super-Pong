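; PongArena is the Pong playfield actor that detects balls entering the two goals and reports scores to the BasePong game mode, cached on BeginPlay.
; Each goal overlap decrements the BallSpawner's BallsInPlay, runs its spawn check and destroys the ball.
; It then calls that goal's P1Scored or P2Scored unless the ball is a bomb.
; P1Goal's bomb check reads the ball cast in P2Goal's event, not its own.
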(event `self.ReceiveBeginPlay`
  (bind _asbase_pong (cast `/Game/Blueprints/BasePong` (`GameplayStatics.GetGameMode`)))
  (set `self.Scores` _asbase_pong))

(event `self.P1Goal.OnComponentBeginOverlap`
  (params (OverlappedComponent :type "PrimitiveComponent Object Reference") (OtherActor :type "Actor Object Reference") (OtherComp :type "PrimitiveComponent Object Reference") (OtherBodyIndex :type Integer) (bFromSweep :type Boolean) (SweepResult :type "HitResult Structure (by ref)"))
  (bind _ballspawner (`self.BallSpawner`))
  (bind _aspong_ball (cast `/Game/Blueprints/PongBall` OtherActor))
  (bind _result (`/Engine/EditorBlueprintResources/StandardMacros.DecrementInt` (`/Game/Blueprints/BallSpawner.BallsInPlay` _ballspawner))
    (:`  `
      (set `/Game/Blueprints/BallSpawner.BallsInPlay` _result _ballspawner)
      (`/Game/Blueprints/BallSpawner.BallSpawnCheck` _ballspawner)
      (`self.K2_DestroyActor` _aspong_ball)
      (if (not (`/Game/Blueprints/PongBall.isBomb` (stale `self.P2Goal.OnComponentBeginOverlap` _aspong_ball)))
        (`/Game/Blueprints/BasePong.P1 Scored` (`self.Scores`))))))

(event `self.P2Goal.OnComponentBeginOverlap`
  (params (OverlappedComponent :type "PrimitiveComponent Object Reference") (OtherActor :type "Actor Object Reference") (OtherComp :type "PrimitiveComponent Object Reference") (OtherBodyIndex :type Integer) (bFromSweep :type Boolean) (SweepResult :type "HitResult Structure (by ref)"))
  (bind _ballspawner (`self.BallSpawner`))
  (bind _aspong_ball (cast `/Game/Blueprints/PongBall` OtherActor))
  (bind _result (`/Engine/EditorBlueprintResources/StandardMacros.DecrementInt` (`/Game/Blueprints/BallSpawner.BallsInPlay` _ballspawner))
    (:`  `
      (set `/Game/Blueprints/BallSpawner.BallsInPlay` _result _ballspawner)
      (`/Game/Blueprints/BallSpawner.BallSpawnCheck` _ballspawner)
      (`self.K2_DestroyActor` _aspong_ball)
      (if (not (`/Game/Blueprints/PongBall.isBomb` _aspong_ball))
        (`/Game/Blueprints/BasePong.P2 Scored` (`self.Scores`))))))

(fn `UserConstructionScript`)